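; GM_Gameplay is a game mode that runs a countdown timer for the match and ends it when time runs out.
; Each tick subtracts delta seconds from GameTimeRemaining and calls TimeCheck.
; At zero or below, TimeCheck creates the W_GameOver widget for player 0, adds it to the viewport and pauses the game.
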(event Custom|TimeCheck
  ;[1 1 1] Time Check ( )
  (if (<= (Variables|Default|GetgameTimeRemaining) 0.0)
    (bind _returnvalue (UserInterface|CreateWidget "/Game/UI/HUD/W_GameOver.W_GameOver_C" (Game|GetPlayerController 0)))
    (UserInterface|Viewport|AddtoViewport _returnvalue 0)
    (Game|SetGamePaused true)))

(event EventTick
  (params (DeltaSeconds :type Float%20%28single-precision%29))
  ;[1 1 1] Tick ( )
  (Variables|Default|SetgameTimeRemaining (- (Variables|Default|GetgameTimeRemaining) DeltaSeconds))
  (CallFunction|TimeCheck))

(fn ConstructionScript)
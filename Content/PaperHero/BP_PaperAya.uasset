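; Paper2D player character Aya, who can drag physics objects with the mouse and open the pause menu.
; While GrabMode is on, the Gun input traces under the cursor and grabs movable, simulating components with a PhysicsHandle, releasing on button up.
; Tick drags the held component along the cursor ray at its original hit distance and picks idle or moving flipbooks from IsMoving and Direction.
; Q prints GrabMode for debugging.
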(event Custom|UpdatePhysicsHandle
  (bind _returnvalue (Game|GetPlayerController 0))
  (bind (_worldlocation _worlddirection) (Game|Player|ConvertMouseLocationToWorldSpace _returnvalue))
  ;[1 1 1] Click and Drag Updater
  (if (and (Variables|Default|GetbGrabMode) (Physics|IsSimulatingPhysics (Variables|Default|GetgrabbedComponent) "None"))
    (Physics|Components|PhysicsHandle|SetTargetLocation (Variables|Default|GetPhysicsHandle) (+ _worldlocation (* _worlddirection (Variables|Default|GetOGDistanceToObj))))))

(event Custom|SetIdleAnimation
  (params (facingDirection :type Direction%20Enum :default "Left"))
  ;[1 1 1] Handling Flipbook Animations
  (Sprite|SetFlipbook (Variables|Default|GetSprite) (Utilities|Select :Index facingDirection :Left "/Game/PaperHero/Sprite/F_Aya_Idle_L.F_Aya_Idle_L" :Right "/Game/PaperHero/Sprite/F_Aya_Idle_R.F_Aya_Idle_R")))

(event Custom|SetMovingAnimation
  (params (facingDirection :type Direction%20Enum :default "Left"))
  ;[1 1 1] Handling Flipbook Animations
  (Sprite|SetFlipbook (Variables|Default|GetSprite) (Utilities|Select :Index facingDirection :Left "/Game/PaperHero/Sprite/F_Aya_Move_L.F_Aya_Move_L" :Right "/Game/PaperHero/Sprite/F_Aya_Move_R.F_Aya_Move_R")))

(event EventTick
  (params (DeltaSeconds :type Float%20%28single-precision%29))
  (bind _direction (Variables|Default|Getdirection))
  ;[1 1 1] Tick ( )
  (Utilities|IsValid (Variables|Default|GetgrabbedComponent)
    (:Is%20Valid
      (CallFunction|UpdatePhysicsHandle))
    (:Is%20Not%20Valid
      _))
  (if (Variables|Default|GetbIsMoving)
    (CallFunction|SetMovingAnimation _direction)
    (else
      (CallFunction|SetIdleAnimation _direction))))

(event Input|ActionEvents|InputActionGun
  (params (Key :type Key%20Structure :default "None"))
  (bind _returnvalue (Game|GetPlayerController 0))
  (bind _bgrabmode (Variables|Default|GetbGrabMode))
  (bind (_worldlocation _worlddirection) (Game|Player|ConvertMouseLocationToWorldSpace _returnvalue))
  ;[1 1 1] Gun
  (:Pressed
    (if _bgrabmode
      (bind (_outhit _returnvalue_2) (Collision|LineTraceByChannel _worldlocation (+ _worldlocation (* _worlddirection (Math|Float|MakeLiteralFloat 1e+05))) "TraceTypeQuery1" true 0 "None"))
      (if _returnvalue_2
        (if (== (Variables|/Script/Engine.SceneComponent|GetMobility (.HitComponent (Collision|BreakHitResult _outhit))) (Utilities|Enum|LiteralenumEComponentMobility "Movable"))
          (Variables|Default|SetOGDistanceToObj (.Distance (Collision|BreakHitResult _outhit)))
          (bind _output_get (Variables|Default|SetgrabbedComponent (.HitComponent (Collision|BreakHitResult _outhit))))
          (if (Physics|IsSimulatingPhysics _output_get "None")
            (Class|PhysicsHandleComponent|GrabComponentatLocation (Variables|Default|GetPhysicsHandle) (Variables|Default|GetgrabbedComponent) "None" (.Location (Collision|BreakHitResult _outhit))))))))
  (:Released
    (if _bgrabmode
      (Variables|Default|SetgrabbedComponent 0)
      (Physics|Components|PhysicsHandle|ReleaseComponent (Variables|Default|GetPhysicsHandle)))))

(event Input|ActionEvents|InputActionPause
  (params (Key :type Key%20Structure :default "None"))
  ;[1 1 1] Pause Menu
  (:Pressed
    (Game|SetGamePaused true)
    (bind _returnvalue (UserInterface|CreateWidget "/Game/UI/HUD/W_PauseMenu.W_PauseMenu_C" (Game|GetPlayerController 0)))
    (bind _output_get (Variables|Default|SetPauseMenu _returnvalue))
    (UserInterface|Viewport|AddtoViewport _output_get 0)))

(event Input|KeyboardEvents|Q
  (params (Key :type Key%20Structure :default "None"))
  (:Pressed
    (Development|PrintString (Utilities|String|Append "Grab Mode: " (Utilities|String|ToString(Boolean) (Variables|Default|GetbGrabMode))))))

(fn ConstructionScript)